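; Blueprint function library that draws a spline component as debug lines and points for a set duration.
; DrawDebugSpline loops over the spline points, drawing each point and calling DrawCurveForSeconds for its segment, wrapping to the first point on closed loops.
; Segments are sampled through GetLocationBezier, a cubic Bézier built from nested lerps.
; Anchors come from tangents scaled by one third for Curve points and zero for other types, with drawing raised by line thickness.
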(fn GetLocationBezier
  (params (StartPoint :type Vector) (AnchorStart :type Vector) (AnchorEnd :type Vector) (EndPoint :type Vector) (Time :type Float%20%28double-precision%29) (__WorldContext :type Object%20Object%20Reference))
  (Utilities|FlowControl|Sequence
    (:then_0
      (LocalVariables|SetTemp_A (Math|Vector|Lerp(Vector) StartPoint AnchorStart Time))
      (LocalVariables|SetTemp_B (Math|Vector|Lerp(Vector) AnchorStart AnchorEnd Time))
      (LocalVariables|SetTemp_C (Math|Vector|Lerp(Vector) AnchorEnd EndPoint Time)))
    (:then_1
      (LocalVariables|SetTemp_D (Math|Vector|Lerp(Vector) (LocalVariables|GetTemp_A) (LocalVariables|GetTemp_B) Time))
      (LocalVariables|SetTemp_E (Math|Vector|Lerp(Vector) (LocalVariables|GetTemp_B) (LocalVariables|GetTemp_C) Time)))
    (:then_2
      (return (Math|Vector|Lerp(Vector) (LocalVariables|GetTemp_D) (LocalVariables|GetTemp_E) Time)))))

(fn DrawCurveforSeconds
  (params (Spline :type Spline%20Component%20Object%20Reference) (Index :type Integer) (SplineColor :type Linear%20Color%20Structure) (Duration :type Float%20%28double-precision%29) (Thickness :type Float%20%28double-precision%29) (__WorldContext :type Object%20Object%20Reference))
  (bind _returnvalue (Spline|GetLocationatSplinePoint Spline Index "World"))
  (bind _returnvalue_2 (Class|SplineComponent|GetSplinePointType Spline Index))
  (bind _returnvalue_3 (Spline|GetNumberOfSplinePoints Spline))
  (bind _returnvalue_4 (+ Index 1))
  (bind _returnvalue_5 (- _returnvalue_3 1))
  (bind _returnvalue_6 (Utilities|Select :Index _returnvalue_2 :Linear 0.0 :Curve 0.333333 :Constant 0.0 :CurveClamped 0.0 :CurveCustomTangent 0.0))
  (bind _returnvalue_7 (< Index _returnvalue_5))
  (bind _returnvalue_8 (select _returnvalue_7 _returnvalue_4 0))
  (bind _returnvalue_9 (Spline|GetLocationatSplinePoint Spline _returnvalue_8 "World"))
  (if (Class|SplineComponent|IsClosedLoop Spline)
    (LocalVariables|SetTemp_DebugStart (+ _returnvalue (Math|Vector|MakeVector 0.0 0.0 Thickness)) :!label _label)
    (while (Math|Float|InRange(Float) (LocalVariables|GetTemp_Time) 0.0 1.01)
      (Utilities|FlowControl|Sequence
        (:then_0
          (LocalVariables|SetTemp_DebugEnd (+ (Math|GetLocationBezier _returnvalue (+ _returnvalue (* (Spline|GetLeaveTangentatSplinePoint Spline Index "World") _returnvalue_6)) (- _returnvalue_9 (* (Spline|GetArriveTangentatSplinePoint Spline _returnvalue_8 "World") _returnvalue_6)) _returnvalue_9 (LocalVariables|GetTemp_Time) __WorldContext) (Math|Vector|MakeVector 0.0 0.0 Thickness)))
          (Rendering|Debug|DrawDebugLine __WorldContext (LocalVariables|GetTemp_DebugStart) (LocalVariables|GetTemp_DebugEnd) SplineColor Duration Thickness)
          (LocalVariables|SetTemp_DebugStart (LocalVariables|GetTemp_DebugEnd)))
        (:then_1
          ;[0 0 0] Simulate the increase of time in the while loop
          (LocalVariables|SetTemp_Time (+ (LocalVariables|GetTemp_Time) 0.05)))))
    (elif (< Index (- (Spline|GetNumberOfSplinePoints Spline) 1))
      (goto _label))))

(fn DrawDebugSpline
  (params (Spline :type Spline%20Component%20Object%20Reference) (SplineColor :type Linear%20Color%20Structure) (PointColor :type Linear%20Color%20Structure :default "(R=0.000000,G=0.000000,B=0.000000,A=1.000000)") (Thickness :type Float%20%28double-precision%29) (PointSize :type Float%20%28single-precision%29) (Duration :type Float%20%28double-precision%29) (__WorldContext :type Object%20Object%20Reference))
  (for _index (range 0 (- (Spline|GetNumberOfSplinePoints Spline) 1))
    (LocalVariables|SetIndex _index)
    (Math|DrawCurveforSeconds Spline (LocalVariables|GetIndex) SplineColor Duration Thickness __WorldContext)
    (Rendering|Debug|DrawDebugPoint __WorldContext (+ (Spline|GetLocationatSplinePoint Spline (LocalVariables|GetIndex) "World") (Math|Vector|MakeVector 0.0 0.0 Thickness)) PointSize PointColor Duration)))